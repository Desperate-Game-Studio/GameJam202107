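; BP_Ball is a physics-driven ball that also carries the end-of-game handling.
; It turns on physics simulation for its mesh at BeginPlay.
; Its HandleGame event pauses the game, creates the victory or game-over widget according to the Result flag, and switches the first player to UI-only input with a visible cursor.
; The file contains no call to HandleGame, and its overlap and tick events are empty.
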(event `self.ReceiveBeginPlay`
  (`PrimitiveComponent.SetSimulatePhysics` (`self.Mesh`) true))

(event `self.HandleGame`
  (params (result :type Boolean))
  (bind _returnvalue (`GameplayStatics.GetPlayerController` 0))
  (bind _returnvalue_2 (`GameplayStatics.GetPlayerController` 0))
  (`GameplayStatics.SetGamePaused` true)
  (`WidgetBlueprintLibrary.SetInputMode_UIOnlyEx` (`GameplayStatics.GetPlayerController` 0) null "LockInFullscreen")
  (if result
    (bind _returnvalue_3 (`|CreateWidget` "/Game/Gamemenu/WB_GameVictory.WB_GameVictory_C" _returnvalue))
    (`UserWidget.AddToViewport` _returnvalue_3 0)
    (else
      (bind _returnvalue_4 (`|CreateWidget` "/Game/Gamemenu/WB_GameOver.WB_GameOver_C" _returnvalue))
      (`UserWidget.AddToViewport` _returnvalue_4 0)))
  (set `PlayerController.bShowMouseCursor` true _returnvalue_2)
  (`WidgetBlueprintLibrary.SetInputMode_UIOnlyEx` _returnvalue_2 null "LockInFullscreen"))

(fn `UserConstructionScript`)